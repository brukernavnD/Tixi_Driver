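; Client pickup actor that marks itself as picked up and removes itself from the level.
; The PickClient event sets IfPickUp, prints a confirmation, then destroys the actor on the next tick.
; A disconnected branch, which never runs, would spawn BP_TheClient at the Cube's transform with a walk/run animation, or destroy it once picked up.
; BeginPlay and the construction script are empty.
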(event Collision|EventActorBeginOverlap
  (params (OtherActor :type Actor%20Object%20Reference)))

(event EventPickClient
  (Variables|Default|Setif%20pick%20up true)
  (Development|PrintString "got it")
  (Utilities|FlowControl|DelayUntilNextTick)
  (Actor|DestroyActor))

(event EventBeginPlay)

(fn ConstructionScript)